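; Shared camera actor that keeps four local player characters in view by following their midpoint and zooming with their spread.
; After a short startup delay it caches the players, then each tick moves a Box to their averaged position.
; The spring arm eases toward that Box on X and Y with a Y offset, holding its starting height.
; Arm length eases toward the largest pairwise player distance, offset and clamped.
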(event `self.ReceiveBeginPlay`
  (bind (_returnvalue_x _returnvalue_y _returnvalue_z) (`KismetMathLibrary.BreakVector` (`self.K2_GetActorLocation`)))
  (bind (_returnvalue_x_2 _returnvalue_y_2) (`KismetMathLibrary.BreakVector` (`SceneComponent.K2_GetComponentLocation` (`self.SpringArm`))))
  ;[1 1 1] Begin play
  (`self.SetActorTickEnabled` false)
  (`KismetSystemLibrary.Delay` 0.2)
  (`self.SetActorTickEnabled` true)
  (`|ExecutionSequence`
    (:`then_0`
      (set `self.Player1` (`GameplayStatics.GetPlayerCharacter` 0))
      (set `self.Player2` (`GameplayStatics.GetPlayerCharacter` 1))
      (set `self.Player3` (`GameplayStatics.GetPlayerCharacter` 2))
      (set `self.player4` (`GameplayStatics.GetPlayerCharacter` 3)))
    (:`then_1`
      (set `self.CameraXPosition` _returnvalue_x_2)
      (set `self.CameraYPosition` _returnvalue_y_2)
      (set `self.StartingPosition` (`KismetMathLibrary.MakeVector` 0.0 0.0 _returnvalue_z)))))

(event `FindHighestDist`
  (bind _player1 (`self.Player1`))
  (bind _player2 (`self.Player2`))
  (bind _player3 (`self.Player3`))
  (bind _player4 (`self.player4`))
  ;[1 1 1] Find Highest distance between two players
  (set `self.HighestDistance` (- (`.MaxValue` (`KismetMathLibrary.MaxOfFloatArray` (`|MakeArray` (`self.GetDistanceTo` _player1 _player2) (`self.GetDistanceTo` _player1 _player3) (`self.GetDistanceTo` _player1 _player4) (`self.GetDistanceTo` _player2 _player3) (`self.GetDistanceTo` _player2 _player4) (`self.GetDistanceTo` _player3 _player4)))) 1300.0)))

(event `SetCollision`
  ;[1 1 1] Set collision position
  (`SceneComponent.K2_SetWorldLocation` (`self.Box`) (`self.NewCameraPosition`) false false))

(event `MoveCamera`
  (bind (_startingposition_x _startingposition_y _startingposition_z) (`KismetMathLibrary.BreakVector` (`self.StartingPosition`)))
  (bind (_returnvalue_x _returnvalue_y) (`KismetMathLibrary.BreakVector` (`SceneComponent.K2_GetComponentLocation` (`self.Box`))))
  ;[1 1 1] Move camera on the X and Y axis
  (set `self.CameraYPosition` (`KismetMathLibrary.FInterpTo` (`self.CameraYPosition`) (- _returnvalue_y (`self.CameraOffset`)) (`self.Delta Seconds`) 0.5))
  (set `self.CameraXPosition` (`KismetMathLibrary.FInterpTo` (`self.CameraXPosition`) _returnvalue_x (`self.Delta Seconds`) 0.5))
  (`SceneComponent.K2_SetWorldLocation` (`self.SpringArm`) (`KismetMathLibrary.MakeVector` (`self.CameraXPosition`) (`self.CameraYPosition`) _startingposition_z) false false))

(event `Set camera position`
  ;[1 1 1] Set new camera position
  (set `self.NewCameraPosition` (/ (+ (`self.K2_GetActorLocation` (`self.Player1`)) (`self.K2_GetActorLocation` (`self.Player2`)) (`self.K2_GetActorLocation` (`self.Player3`)) (`self.K2_GetActorLocation` (`self.player4`))) (4.0 4.0 4.0))))

(event `Zoom`
  (bind _springarm (`self.SpringArm`))
  ;[1 1 1] Zoom the camera on the players
  (set `SpringArmComponent.TargetArmLength` (`KismetMathLibrary.FInterpTo` (`SpringArmComponent.TargetArmLength` _springarm) (`KismetMathLibrary.FMax` (`KismetMathLibrary.FMin` (`self.HighestDistance`) 800.0)) (`self.Delta Seconds`) 0.7) _springarm))

(event `self.ReceiveTick`
  (params (DeltaSeconds :type "Float (single-precision)"))
  ;[1 1 1] Tick
  (set `self.Delta Seconds` DeltaSeconds)
  (`self.FindHighestDist`)
  (`self.Set camera position`)
  (`self.Zoom`)
  (`self.SetCollision`)
  (`self.MoveCamera`))

(fn `UserConstructionScript`)