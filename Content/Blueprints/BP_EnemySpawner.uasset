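; Enemy spawner actor that keeps topping up the level's MeleeEnemy population while fewer than eight exist.
; Tick counts all MeleeEnemy actors in the world every frame and calls Spawnennemy when the count is below the cap.
; That event's two-second Delay ignores repeat calls while pending, pacing spawns before an AI pawn appears at a random point inside the SpawnZone box.
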(event `Spawn ennemy`
  (bind _spawnzone (`self.SpawnZone`))
  (`KismetSystemLibrary.Delay` 2.0)
  (`AIBlueprintHelperLibrary.SpawnAIFromClass` "/Game/Blueprints/Enemy/MeleeEnemy.MeleeEnemy_C" null (`KismetMathLibrary.RandomPointInBoundingBox` (`SceneComponent.K2_GetComponentLocation` _spawnzone) (`BoxComponent.GetScaledBoxExtent` _spawnzone)) (struct) false null))

(event `self.ReceiveTick`
  (params (DeltaSeconds :type "Float (single-precision)"))
  (bind _outactors (`GameplayStatics.GetAllActorsOfClass` "/Game/Blueprints/Enemy/MeleeEnemy.MeleeEnemy_C"))
  (if (< (`KismetArrayLibrary.Array_Length` _outactors) 8)
    (`self.Spawn ennemy`)))

(fn `UserConstructionScript`)