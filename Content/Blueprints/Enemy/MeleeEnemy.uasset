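; Melee enemy that chases players and attacks them in close range, with a death sequence of sound, animation and destruction.
; Each Tick scans all BP_ConnectionPlayer actors for the two nearest, keeping stored distances that are never reset here.
; It AI-moves to the nearest, or the runner-up if that player is dead.
; On arrival it damages the player and updates their health bar, gated by an attack-rate cooldown.
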(event `EnemyDeath`
  (set `self.canAttack?` false)
  (`CharacterMovementComponent.DisableMovement` (`self.CharacterMovement`))
  (`GameplayStatics.PlaySound2D` "/Game/Sounds/deathsoundEnemy.deathsoundEnemy" 1.0 1.0 0.0 null null)
  (`SkeletalMeshComponent.PlayAnimation` (`self.Mesh`) "/Game/ModularRPGHeroesPolyart/Animations/NoWeaponStance/Die_noWeaponAnim.Die_noWeaponAnim" false)
  (`KismetSystemLibrary.Delay` 1.0)
  (`self.K2_DestroyActor`))

(event `self.ReceiveBeginPlay`)

(event `self.ReceiveTick`
  (params (DeltaSeconds :type "Float (single-precision)"))
  (`self.GetClosestPlayer`)
  (`self.ChasePlayer`))

(event `ChasePlayer`
  (bind _closestplayer (`self.closestPlayer`))
  (bind _closestplayer_2 (`self.closestPlayer`))
  (if (`/Game/Blueprints/BP_ConnectionPlayer.isPlayerDead` _closestplayer)
    (set `self.closestPlayer` (`self.secondClosestPlayer`)))
  (`|AIMoveTo` self (0.0 0.0 0.0) _closestplayer (`self.attackRange`)
    (:`OnSuccess`
      (if (`self.canAttack?`)
        (set `self.canAttack?` false)
        (bind _currenthp (`/Game/Blueprints/BP_ConnectionPlayer.ModifyHealth` _closestplayer_2 (`self.Damage`)))
        (`/Game/Blueprints/PlayerHealthBar.UpdateHealth` (`/Game/Blueprints/BP_ConnectionPlayer.As Player Health Bar` _closestplayer_2) _currenthp)
        (`KismetSystemLibrary.Delay` (`self.attackRate`))
        (set `self.canAttack?` true)))))

(fn `GetClosestPlayer`
  (bind _outactors (`GameplayStatics.GetAllActorsOfClass` "/Game/Blueprints/BP_ConnectionPlayer.BP_ConnectionPlayer_C"))
  (for _array_element _outactors
    (bind _returnvalue (`self.GetDistanceTo` _array_element))
    (if (<= _returnvalue (`self.closestDistance`))
      (set `self.closestPlayer` _array_element)
      (set `self.closestDistance` _returnvalue)
      (elif (<= _returnvalue (`self.secondClosestDistance`))
        (set `self.secondClosestPlayer` _array_element)
        (set `self.secondClosestDistance` _returnvalue)))))

(fn `UserConstructionScript`)