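; BP_PlayerRefillIndicator is a compass-style cone that orbits a player and points toward that player's safe zone refiller.
; After a one-second delay it finds the BP_ConnectionPlayer and BP_SafeZoneRefiller whose IDs match CompassId, caching the refiller's location once.
; Each Tick computes the planar player-to-refiller angle with atan2, places the actor at Radius around the player, and yaws the cone toward the target.
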(event `self.ReceiveBeginPlay`
  (`KismetSystemLibrary.Delay` 1.0)
  (bind _outactors (`GameplayStatics.GetAllActorsOfClass` "/Game/Blueprints/BP_ConnectionPlayer.BP_ConnectionPlayer_C"))
  (for _array_element _outactors
    (if (== (`/Game/Blueprints/BP_ConnectionPlayer.PlayerID` _array_element) (`self.CompassId`))
      (bind _output_get (set `self.Player` _array_element))
      (`self.K2_SetActorTransform` (`self.GetTransform` _output_get) false true)
      (`self.FindCrystalFiller`))))

(event `FindCrystalFiller`
  (bind _outactors (`GameplayStatics.GetAllActorsOfClass` "/Game/Blueprints/BP_SafeZoneRefiller.BP_SafeZoneRefiller_C"))
  (for _array_element _outactors
    (if (== (`/Game/Blueprints/BP_SafeZoneRefiller.IdRefiller` _array_element) (`self.CompassId`))
      (set `self.TargetLocation` (`self.K2_GetActorLocation` _array_element)))))

(event `self.ReceiveTick`
  (params (DeltaSeconds :type "Float (single-precision)"))
  (`/Engine/EditorBlueprintResources/StandardMacros.IsValid` (`self.Player`)
    (:`Is Valid`
      (`self.FindAngle`)
      (`self.ActorRotator` (`self.Player`)))))

(event `FindAngle`
  (bind (_targetlocation_x _targetlocation_y) (`KismetMathLibrary.BreakVector` (`self.TargetLocation`)))
  (bind (_returnvalue_x _returnvalue_y) (`KismetMathLibrary.BreakVector` (`self.K2_GetActorLocation` (`self.Player`))))
  (set `self.AngleBetweenCharacterAndRefill` (`KismetMathLibrary.DegAtan2` (- _targetlocation_x _returnvalue_x) (- _targetlocation_y _returnvalue_y))))

(fn `ActorRotator`
  (params (Target :type "Actor Object Reference"))
  (bind _returnvalue (+ (`self.LocalLocation`) (`KismetMathLibrary.RotateAngleAxis` (`KismetMathLibrary.MakeVector` 0.0 (`self.Radius`)) (- (`self.StartAngle`) (`self.AngleBetweenCharacterAndRefill`)) (0.0 0.0 1.0))))
  (bind (_returnvalue_roll _returnvalue_pitch _returnvalue_yaw) (`KismetMathLibrary.BreakRotator` (`KismetMathLibrary.FindLookAtRotation` _returnvalue (`self.TargetLocation`))))
  (set `self.LocalLocation` (`self.K2_GetActorLocation` Target))
  (`self.K2_SetActorLocation` _returnvalue)
  (`SceneComponent.K2_SetWorldRotation` (`self.Cone`) (`KismetMathLibrary.MakeRotator` _returnvalue_roll 270.0 _returnvalue_yaw) false false))

(fn `UserConstructionScript`)