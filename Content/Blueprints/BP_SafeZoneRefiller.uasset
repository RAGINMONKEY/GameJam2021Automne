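; BP_SafeZoneRefiller is a per-player safe-zone refill station, paired by IdRefiller.
; On BeginPlay it teleports to the TargetPoint tagged "R" plus its ID, then after a short delay caches the BP_ConnectionPlayer with the matching PlayerID.
; Its box overlap events are empty; the logic toggling InRefillArea, CanRefill and SafeZoneAOE recharging is disconnected and never runs.
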(event `self.ReceiveBeginPlay`
  (`self.Spawn`)
  (`KismetSystemLibrary.Delay` 0.2)
  (bind _outactors (`GameplayStatics.GetAllActorsOfClass` "/Game/Blueprints/BP_ConnectionPlayer.BP_ConnectionPlayer_C"))
  (for _array_element _outactors
    (if (== (`self.IdRefiller`) (`/Game/Blueprints/BP_ConnectionPlayer.PlayerID` _array_element))
      (set `self.Player` _array_element))))

(event `self.Box.OnComponentBeginOverlap`
  (params (OverlappedComponent :type "PrimitiveComponent Object Reference") (OtherActor :type "Actor Object Reference") (OtherComp :type "PrimitiveComponent Object Reference") (OtherBodyIndex :type Integer) (bFromSweep :type Boolean) (SweepResult :type "HitResult Structure (by ref)")))

(event `self.Box.OnComponentEndOverlap`
  (params (OverlappedComponent :type "PrimitiveComponent Object Reference") (OtherActor :type "Actor Object Reference") (OtherComp :type "PrimitiveComponent Object Reference") (OtherBodyIndex :type Integer)))

(fn `Spawn`
  (bind _outactors (`GameplayStatics.GetAllActorsOfClassWithTag` "/Script/Engine.TargetPoint" (`KismetStringLibrary.Conv_StringToName` (`KismetStringLibrary.Concat_StrStr` "R" (`KismetStringLibrary.Conv_IntToString` (`self.IdRefiller`))))))
  (`self.K2_SetActorTransform` (`self.GetTransform` (`|GetArrayItem` _outactors)) false true))

(fn `UserConstructionScript`)