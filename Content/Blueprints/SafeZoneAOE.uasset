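; SafeZoneAOE is a per-player safe zone actor with a crystal that stops damage over time for its matching player.
; On BeginPlay it teleports to the TargetPoint tagged "SZ" plus its ID and sets crystal material and beam color by ID.
; Overlap compares PlayerID to ID, toggling damage over time and beam visibility for the owner, or double damage for others.
; While the owner is connected, Tick updates the beam between crystal and player.
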(event `self.ReceiveBeginPlay`
  (bind _particleconnection (`self.ParticleConnection`))
  (bind _crystal (`self.Crystal`))
  (`self.Spawn`)
  (switch `int` (`self.ID`)
    (:`0`
      (`PrimitiveComponent.SetMaterial` _crystal 0 "/Game/CrystalAsset/MaterialRed.MaterialRed")
      (`FXSystemComponent.SetColorParameter` _particleconnection "ParamColor" (make `LinearColor` 0.0 0.0 200.0 200.0)))
    (:`1`
      (`PrimitiveComponent.SetMaterial` _crystal 0 "/Game/CrystalAsset/MaterialBlue.MaterialBlue")
      (`FXSystemComponent.SetColorParameter` _particleconnection "None" (make `LinearColor` 0.0 0.0 1.0)))
    (:`2`
      (`PrimitiveComponent.SetMaterial` _crystal 0 "/Game/CrystalAsset/MaterialGreen.MaterialGreen")
      (`FXSystemComponent.SetColorParameter` _particleconnection "None" (make `LinearColor` 0.0 1.0)))
    (:`3`
      (`PrimitiveComponent.SetMaterial` _crystal 0 "/Game/CrystalAsset/MaterialYellow.MaterialYellow")
      (`FXSystemComponent.SetColorParameter` _particleconnection "None" (make `LinearColor` 1.0 1.0)))))

(event `self.ReceiveActorEndOverlap`
  (params (OtherActor :type "Actor Object Reference"))
  ;[1 1 1] End Overlap
  (bind _asbp_connection_player (cast `/Game/Blueprints/BP_ConnectionPlayer` OtherActor)
    (:`then`
      (if (== (`/Game/Blueprints/BP_ConnectionPlayer.PlayerID` _asbp_connection_player) (`self.ID`))
        (set `/Game/Blueprints/BP_ConnectionPlayer.TakeDmgOverTime` true _asbp_connection_player)
        (set `self.isConnectedToPlayer` false)
        (`SceneComponent.SetVisibility` (`self.ParticleConnection`) false false)
        (else
          (set `/Game/Blueprints/BP_ConnectionPlayer.DoubleDmg` false _asbp_connection_player))))
    (:`CastFailed`
      (`KismetSystemLibrary.PrintString` "ConnectionPlayer cast failed!"))))

(event `self.ReceiveActorBeginOverlap`
  (params (OtherActor :type "Actor Object Reference"))
  ;[1 1 1] Begin Overlap
  (bind _asbp_connection_player (cast `/Game/Blueprints/BP_ConnectionPlayer` OtherActor)
    (:`then`
      (if (== (`/Game/Blueprints/BP_ConnectionPlayer.PlayerID` _asbp_connection_player) (`self.ID`))
        (set `/Game/Blueprints/BP_ConnectionPlayer.TakeDmgOverTime` false _asbp_connection_player)
        (set `self.As BP Connection Player` _asbp_connection_player)
        (set `self.isConnectedToPlayer` true)
        (`SceneComponent.SetVisibility` (`self.ParticleConnection`) true false)
        (else
          (set `/Game/Blueprints/BP_ConnectionPlayer.DoubleDmg` true _asbp_connection_player))))
    (:`CastFailed`
      (`KismetSystemLibrary.PrintString` "ConnectionPlayer cast failed!"))))

(event `self.ReceiveTick`
  (params (DeltaSeconds :type "Float (single-precision)"))
  (if (`self.isConnectedToPlayer`)
    (`ParticleSystemComponent.SetBeamSourcePoint` (`self.ParticleConnection`) 0 (`SceneComponent.K2_GetComponentLocation` (`self.Crystal`)) 0)
    (`ParticleSystemComponent.SetBeamTargetPoint` (`self.ParticleConnection`) 0 (`SceneComponent.K2_GetComponentLocation` (`Character.Mesh` (`self.As BP Connection Player`))) 0)))

(fn `Spawn`
  (bind _outactors (`GameplayStatics.GetAllActorsOfClassWithTag` "/Script/Engine.TargetPoint" (`KismetStringLibrary.Conv_StringToName` (`KismetStringLibrary.Concat_StrStr` "SZ" (`KismetStringLibrary.Conv_IntToString` (`self.ID`))))))
  (`self.K2_SetActorTransform` (`self.GetTransform` (`|GetArrayItem` _outactors)) false true))

(fn `UserConstructionScript`)