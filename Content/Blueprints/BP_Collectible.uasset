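; BP_Collectible is a pickup actor that adds its value to the score of the player who touches it.
; It caches the BP_ConnectionGameInstance on BeginPlay, where scores live in an array indexed by PlayerID.
; When a BP_ConnectionPlayer overlaps the collider, it destroys the collider, hides the mesh, increments that player's score entry and destroys itself.
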(event `self.ReceiveBeginPlay`
  (bind _asbp_connection_game_instance (cast `/Game/Blueprints/BP_ConnectionGameInstance` (`GameplayStatics.GetGameInstance`)))
  (set `self.GameInstance` _asbp_connection_game_instance))

(event `self.Collider.OnComponentBeginOverlap`
  (params (OverlappedComponent :type "PrimitiveComponent Object Reference") (OtherActor :type "Actor Object Reference") (OtherComp :type "PrimitiveComponent Object Reference") (OtherBodyIndex :type Integer) (bFromSweep :type Boolean) (SweepResult :type "HitResult Structure (by ref)"))
  (bind _score (`/Game/Blueprints/BP_ConnectionGameInstance.Score` (`self.GameInstance`)))
  (bind _asbp_connection_player (cast `/Game/Blueprints/BP_ConnectionPlayer` OtherActor))
  (`ActorComponent.K2_DestroyComponent` (`self.Collider`))
  (`SceneComponent.SetVisibility` (`self.StaticMesh`) false false)
  (bind _playerid (`/Game/Blueprints/BP_ConnectionPlayer.PlayerID` _asbp_connection_player))
  (`KismetArrayLibrary.Array_Set` _score _playerid (+ (`|GetArrayItem` _score _playerid) (`self.Value`)))
  (`self.K2_DestroyActor`))

(fn `UserConstructionScript`)