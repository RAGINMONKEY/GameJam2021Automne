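; Spawner actor that replenishes BP_Collectible pickups inside its SpawnZone volume whenever fewer than three exist in the world.
; Tick counts collectibles with GetAllActorsOfClass each frame and calls the Spawnennemy event, which spawns a collectible despite its name.
; That event's Delay ignores repeat calls while pending, throttling spawns to one per ten-second wait, each at a random point in the zone's bounds.
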(event `Spawn ennemy`
  (bind _spawnzone (`self.SpawnZone`))
  (`KismetSystemLibrary.Delay` 10.0)
  (`|SpawnActorFromClass` "/Game/Blueprints/BP_Collectible.BP_Collectible_C" (`KismetMathLibrary.MakeTransform` (`KismetMathLibrary.RandomPointInBoundingBox` (`SceneComponent.K2_GetComponentLocation` _spawnzone) (`BoxComponent.GetScaledBoxExtent` _spawnzone))) "Undefined" "OverrideRootScale" null null))

(event `self.ReceiveTick`
  (params (DeltaSeconds :type "Float (single-precision)"))
  (bind _outactors (`GameplayStatics.GetAllActorsOfClass` "/Game/Blueprints/BP_Collectible.BP_Collectible_C"))
  (if (< (`KismetArrayLibrary.Array_Length` _outactors) 3)
    (`self.Spawn ennemy`)))

(fn `UserConstructionScript`)