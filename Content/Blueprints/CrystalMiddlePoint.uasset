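; CrystalMiddlePoint is the center trigger of a SafeZoneAOE that controls whether that safe zone is recharging.
; On BeginPlay it casts its parent actor to SafeZoneAOE, copies the zone's ID and registers itself as the zone's middle point.
; Overlap with a BP_SafeZoneRefiller whose ID matches sets the zone's IsRecharging, and ending that overlap clears it, with debug prints along the way.
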(event `self.ReceiveBeginPlay`
  (bind _assafe_zone_aoe (cast `/Game/Blueprints/SafeZoneAOE` (`self.GetParentActor`)))
  (set `self.id` (`/Game/Blueprints/SafeZoneAOE.ID` _assafe_zone_aoe))
  (set `/Game/Blueprints/SafeZoneAOE.MiddlePointReference` self _assafe_zone_aoe)
  (set `self.SafeZoneRef` _assafe_zone_aoe))

(event `self.ReceiveActorBeginOverlap`
  (params (OtherActor :type "Actor Object Reference"))
  (`KismetSystemLibrary.PrintString` "goes in")
  (bind _asbp_safe_zone_refiller (cast `/Game/Blueprints/BP_SafeZoneRefiller` OtherActor))
  (if (== (`self.id`) (`/Game/Blueprints/BP_SafeZoneRefiller.IdRefiller` _asbp_safe_zone_refiller))
    (set `/Game/Blueprints/SafeZoneAOE.isRecharging` true (`self.SafeZoneRef`))
    (`KismetSystemLibrary.PrintString` "recharge")))

(event `self.ReceiveActorEndOverlap`
  (params (OtherActor :type "Actor Object Reference"))
  (bind _asbp_safe_zone_refiller (cast `/Game/Blueprints/BP_SafeZoneRefiller` OtherActor))
  (if (== (`self.id`) (`/Game/Blueprints/BP_SafeZoneRefiller.IdRefiller` _asbp_safe_zone_refiller))
    (set `/Game/Blueprints/SafeZoneAOE.isRecharging` false (`self.SafeZoneRef`))
    (`KismetSystemLibrary.PrintString` "no recharge")))

(fn `UserConstructionScript`)