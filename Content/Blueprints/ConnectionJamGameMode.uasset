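; Game mode for Connection Jam that sets up a local multiplayer match with one shared camera.
; On BeginPlay it reads the player count from BP_ConnectionGameInstance, creates the extra local players, then spawns and possesses a BP_ConnectionPlayer for each.
; It also spawns a SafeZoneAOE and BP_SafeZoneRefiller per player, linked by index ID, all at one fixed location.
; It then blends player 0's view to the first ConnectionCamera found.
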(event `self.ReceiveBeginPlay`
  (bind _asbp_connection_game_instance (cast `/Game/Blueprints/BP_ConnectionGameInstance` (`GameplayStatics.GetGameInstance`)))
  (set `self.GameInstance` _asbp_connection_game_instance)
  (`|ExecutionSequence`
    (:`then_0`
      (`self.SpawnPlayers`)
      (`self.FindCamera`))
    (:`then_1`
      (`PlayerController.SetViewTargetWithBlend` (`GameplayStatics.GetPlayerController` 0) (`self.GameCamera`) 0.0 "VTBlend_Linear" 0.0 false))))

(event `FindCamera`
  (bind _outactors (`GameplayStatics.GetAllActorsOfClass` "/Game/Blueprints/ConnectionCamera.ConnectionCamera_C"))
  (set `self.GameCamera` (`|GetArrayItem` _outactors)))

(fn `SpawnPlayers`
  (bind _returnvalue (- (`/Game/Blueprints/BP_ConnectionGameInstance.PlayerNumber` (`self.GameInstance`)) 1))
  ;[1 1 1] Spawn player and his elements in the game
  (for _index (range 1 (+ _returnvalue 1))
    (`GameplayStatics.CreatePlayer` _index))
  (for _index_2 (range (+ _returnvalue 1))
    (bind _returnvalue_2 (`|SpawnActorFromClass` "/Game/Blueprints/BP_ConnectionPlayer.BP_ConnectionPlayer_C" (`KismetMathLibrary.MakeTransform` (0.0 0.0 2000.0)) "Undefined" "OverrideRootScale" null _index_2 null))
    (`Controller.Possess` (`GameplayStatics.GetPlayerController` _index_2) _returnvalue_2))
  (for _index_3 (range (+ _returnvalue 1))
    (`|SpawnActorFromClass` "/Game/Blueprints/SafeZoneAOE.SafeZoneAOE_C" (`KismetMathLibrary.MakeTransform` (0.0 0.0 2000.0)) "Undefined" "OverrideRootScale" null _index_3 null))
  (for _index_4 (range (+ _returnvalue 1))
    (`|SpawnActorFromClass` "/Game/Blueprints/BP_SafeZoneRefiller.BP_SafeZoneRefiller_C" (`KismetMathLibrary.MakeTransform` (0.0 0.0 2000.0)) "Undefined" "OverrideRootScale" null _index_4 null)))

(fn `UserConstructionScript`)